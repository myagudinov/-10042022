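; Health component that tracks an actor's current health and reports changes and death.
; Health starts at MaxHealth on BeginPlay and is exposed through a getter.
; ApplyDamage subtracts damage clamped at zero, fires the OnChange dispatcher, and calls the Death dispatcher through a DoOnce when health reaches zero.
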(event `self.ReceiveBeginPlay`
  (set `self.Health` (`self.MaxHealth`)))

(fn `Apply Damage`
  (params (Damage :type "Float (double-precision)"))
  (bind _output_get (set `self.Health` (`KismetMathLibrary.FMax` (- (`self.Health`) (`local.Damage`)))))
  (`self.OnChange`)
  (if (== _output_get 0.0)
    (`/Engine/EditorBlueprintResources/StandardMacros.DoOnce` false
      (:`Completed`
        (`self.Death`)))))

(fn `GetHealth`
  (returns (Health :type "Float (double-precision)"))
  (return (`self.Health`)))